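; BP_Pount is a puzzle point actor that detects whether a BP_Pawn sits above it and whether their color selections match.
; On BeginPlay its Selection sets the plane material, with the Close option also enabling collision on its box.
; Each tick an upward Visibility line trace with debug drawing updates Clear for occupancy and, when a pawn is hit, SelfColor by comparing both selections as text.
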(event EventBeginPlay
  (switch Utilities|FlowControl|Switch|SwitchonE_Type (Variables|Default|GetSelection)
    (:NewEnumerator0
      (Rendering|Material|SetMaterial (Variables|Default|GetPlane) 0 "/Engine/VREditor/BasicMeshes/MI_Cube_03.MI_Cube_03"))
    (:NewEnumerator2
      (Rendering|Material|SetMaterial (Variables|Default|GetPlane) 0 "/Engine/MapTemplates/Materials/BasicAsset03.BasicAsset03"))
    (:NewEnumerator3
      (Collision|SetCollisionEnabled (Variables|Default|GetBox) "QueryAndPhysics")
      (Rendering|Material|SetMaterial (Variables|Default|GetPlane) 0 "/Engine/EditorMeshes/ColorCalibrator/M_ClearCoatBlack.M_ClearCoatBlack"))
    (:NewEnumerator4
      (Rendering|Material|SetMaterial (Variables|Default|GetPlane) 0 "/Engine/EngineMaterials/CubeMaterial.CubeMaterial"))))

(event Collision|EventActorBeginOverlap
  (params (OtherActor :type Actor%20Object%20Reference)))

(event EventTick
  (params (DeltaSeconds :type Float%20%28single-precision%29))
  (bind _returnvalue (Transformation|GetActorLocation))
  (bind (_outhit _returnvalue_2) (Collision|LineTraceByChannel _returnvalue (+ _returnvalue (* (Transformation|GetActorUpVector) 200)) "TraceTypeQuery1" false 0 "ForDuration"))
  (if _returnvalue_2
    (bind _asbp_pawn (Utilities|Casting|CastToBP_Pawn (.HitActor (Collision|BreakHitResult _outhit)))
      (:then
        (Variables|Default|SetClear? false)
        (if (Utilities|Enum|Equal(Enum) (Utilities|Text|ToText(String) (Variables|/Game/Puzzle/Blueprints/BP_Pawn.BP_Pawn_C|GetSelection _asbp_pawn)) (Utilities|Text|ToText(String) (Variables|Default|GetSelection)))
          (Variables|Default|SetSelfColor true)
          (else
            (Variables|Default|SetSelfColor false))))
      (:CastFailed
        (Variables|Default|SetClear? true)))
    (else
      (Variables|Default|SetClear? true))))

(fn ConstructionScript)