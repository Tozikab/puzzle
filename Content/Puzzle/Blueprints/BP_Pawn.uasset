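; BP_Pawn is a grid puzzle piece that the player possesses by clicking its cube and moves in fixed steps with WASD.
; On BeginPlay its Selection (Red, Green or Yellow) sets the cube material.
; Before each move, TraceForward or TraceRight line-traces from one step away to two steps away, with debug drawing.
; The move happens only if the trace hits a BP_Pount that is Clear and not set to Close.
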(event OnClicked(Cube)
  (params (TouchedComponent :type Primitive%20Component%20Object%20Reference) (ButtonPressed :type Key%20Structure :default "None"))
  (Pawn|Possess (Game|GetPlayerController 0) self))

(event EventBeginPlay
  (switch Utilities|FlowControl|Switch|SwitchonE_Type (Variables|Default|GetSelection)
    (:NewEnumerator0
      (Rendering|Material|SetMaterial (Variables|Default|GetCube) 0 "/Engine/VREditor/BasicMeshes/MI_Cube_03.MI_Cube_03"))
    (:NewEnumerator2
      (Rendering|Material|SetMaterial (Variables|Default|GetCube) 0 "/Engine/MapTemplates/Materials/BasicAsset03.BasicAsset03"))
    (:NewEnumerator4
      (Rendering|Material|SetMaterial (Variables|Default|GetCube) 0 "/Engine/VREditor/BasicMeshes/MI_Cube_01.MI_Cube_01"))))

(event Collision|EventActorBeginOverlap
  (params (OtherActor :type Actor%20Object%20Reference)))

(event EventTick
  (params (DeltaSeconds :type Float%20%28single-precision%29)))

(event Input|KeyboardEvents|D
  (params (Key :type Key%20Structure :default "None"))
  (:Pressed
    (bind _newparam (CallFunction|TraceRight 100))
    (if _newparam
      (Transformation|SetActorLocation (+ (Transformation|GetActorLocation) (* (Transformation|GetActorRightVector) 100)) false false))))

(event Input|KeyboardEvents|W
  (params (Key :type Key%20Structure :default "None"))
  (:Pressed
    (bind _newparam (CallFunction|TraceForward 100))
    (if _newparam
      (Transformation|SetActorLocation (+ (Transformation|GetActorLocation) (* (Transformation|GetActorForwardVector) 100)) false false))))

(event Input|KeyboardEvents|A
  (params (Key :type Key%20Structure :default "None"))
  (:Pressed
    (bind _newparam (CallFunction|TraceRight -100))
    (if _newparam
      (Transformation|SetActorLocation (+ (Transformation|GetActorLocation) (* (Transformation|GetActorRightVector) -100)) false false))))

(event Input|KeyboardEvents|S
  (params (Key :type Key%20Structure :default "None"))
  (:Pressed
    (bind _newparam (CallFunction|TraceForward -100))
    (if _newparam
      (Transformation|SetActorLocation (+ (Transformation|GetActorLocation) (* (Transformation|GetActorForwardVector) -100)) false false))))

(fn ConstructionScript)

(fn TraceForward
  (params (B :type Integer))
  (bind _returnvalue (Transformation|GetActorLocation))
  (bind _returnvalue_2 (Transformation|GetActorForwardVector))
  (bind _returnvalue_3 (* _returnvalue_2 B))
  (bind _returnvalue_4 (+ _returnvalue _returnvalue_3))
  (bind (_outhit _returnvalue_5) (Collision|LineTraceByChannel _returnvalue_4 (+ _returnvalue_4 (* (Transformation|GetActorForwardVector) B)) "TraceTypeQuery1" false 0 "ForDuration"))
  (bind _asbp_pount (Utilities|Casting|CastToBP_Pount (.HitActor (Collision|BreakHitResult _outhit)))
    (:then
      (if (Math|Boolean|ANDBoolean (not (Utilities|Enum|Equal(Enum) (Variables|/Game/Puzzle/Blueprints/BP_Pount.BP_Pount_C|GetSelection _asbp_pount) "NewEnumerator3")) _returnvalue_5 (Variables|/Game/Puzzle/Blueprints/BP_Pount.BP_Pount_C|GetClear? _asbp_pount))
        (Development|PrintString (Utilities|GetDisplayName (.HitActor (Collision|BreakHitResult _outhit))))
        (return true)
        (else
          _)))
    (:CastFailed
      _))
  (return false))

(fn TraceRight
  (params (B :type Integer))
  (bind _returnvalue (Transformation|GetActorRightVector))
  (bind _returnvalue_2 (Transformation|GetActorLocation))
  (bind _returnvalue_3 (* _returnvalue B))
  (bind _returnvalue_4 (+ _returnvalue_2 _returnvalue_3))
  (bind (_outhit _returnvalue_5) (Collision|LineTraceByChannel _returnvalue_4 (+ _returnvalue_4 (* (Transformation|GetActorRightVector) B)) "TraceTypeQuery1" false 0 "ForDuration"))
  (bind _asbp_pount (Utilities|Casting|CastToBP_Pount (.HitActor (Collision|BreakHitResult _outhit)))
    (:then
      (if (Math|Boolean|ANDBoolean (not (Utilities|Enum|Equal(Enum) (Variables|/Game/Puzzle/Blueprints/BP_Pount.BP_Pount_C|GetSelection _asbp_pount) "NewEnumerator3")) _returnvalue_5 (Variables|/Game/Puzzle/Blueprints/BP_Pount.BP_Pount_C|GetClear? _asbp_pount))
        (Development|PrintString (Utilities|GetDisplayName (.HitActor (Collision|BreakHitResult _outhit))))
        (return true)
        (else
          _)))
    (:CastFailed
      _))
  (return false))